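; Player pawn Blueprint that handles movement and an interact action.
; Forward and right axis inputs, scaled by SpeedMovement, accumulate movement along the actor's forward and right vectors.
; Tick consumes that vector and applies it, scaled by delta time, as a swept local offset, although the input directions are world-space.
; Pressing interact sends InteractMessage to every B_interface_interact actor overlapping the player.
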(event Collision|EventActorBeginOverlap
  (params (OtherActor :type Actor%20Object%20Reference)))

(event EventTick
  (params (DeltaSeconds :type Float%20%28single-precision%29))
  ;[1 1 1] Movement
  ;;[1 1 1] Tick
  (bind _returnvalue (Class|Pawn|ConsumeMovementInputVector))
  (Transformation|AddActorLocalOffset (* _returnvalue DeltaSeconds) true false))

(event Input|ActionEvents|InputActioninteract
  (params (Key :type Key%20Structure :default "None"))
  ;[1 1 1] interact
  ;;[1 1 1] dialogue
  (:Pressed
    (bind _outactors (Actor|GetAllActorswithInterface "/Game/ourProject/UI/B_interface_interact.B_interface_interact_C"))
    (for _array_element _outactors
      (if (Collision|IsOverlappingActor _array_element self :!class /Script/Engine.Actor)
        (Class|BInterfaceInteract|Interact(Message) _array_element)))))

(event Input|AxisEvents|InputAxisMoveForward
  (params (AxisValue :type Float%20%28single-precision%29))
  ;[1 1 1] Movement
  (Pawn|Input|AddMovementInput (Transformation|GetActorForwardVector) (* AxisValue (Variables|Default|Getspeed_movement)) false))

(event Input|AxisEvents|InputAxisMoveRight
  (params (AxisValue :type Float%20%28single-precision%29))
  ;[1 1 1] Movement
  (Pawn|Input|AddMovementInput (Transformation|GetActorRightVector) (* AxisValue (Variables|Default|Getspeed_movement)) false))

(fn ConstructionScript)