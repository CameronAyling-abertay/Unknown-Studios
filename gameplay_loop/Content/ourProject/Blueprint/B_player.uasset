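; Player pawn represented by a two-sided sheep, moved by forward and right axis input.
; Axis events add movement input scaled by MaxSpeed, which Tick consumes and applies as a frame-rate-scaled, swept local offset.
; Tick also steps a clamped half-turn Rotation from an axis value, without delta-time scaling, to spin the Sheep and SheepBack components between front and back.
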(event EventBeginPlay)

(event Collision|EventActorBeginOverlap
  (params (OtherActor :type Actor%20Object%20Reference)))

(event EventTick
  (params (DeltaSeconds :type Float%20%28single-precision%29))
  ;[1 1 1] Tick
  (bind _returnvalue (Class|Pawn|ConsumeMovementInputVector))
  (Transformation|AddActorLocalOffset (* _returnvalue DeltaSeconds) true false)
  ;[1 1 1] Spinning back and front
  (bind _output_get (Variables|Default|SetRotation (Math|Float|Max(Float) (Math|Float|Min(Float) (+ (Variables|Default|GetRotation) (* 2e+01 (stale Input|AxisEvents|InputAxisMoveForward AxisValue))) 1.8e+02) 0.0)))
  (Transformation|SetRelativeRotation (Variables|sprite|GetSheep) (Math|Rotator|MakeRotator 9e+01 0.0 (+ 9e+01 _output_get)) false false)
  (Transformation|SetRelativeRotation (Variables|Default|GetSheepBack) (Math|Rotator|MakeRotator -9e+01 1.8e+02 (+ 9e+01 _output_get)) false false))

(event Input|AxisEvents|InputAxisMoveRight
  (params (AxisValue :type Float%20%28single-precision%29))
  ;[1 1 1] Movement
  (Pawn|Input|AddMovementInput (Transformation|GetActorRightVector) (* AxisValue (Variables|Default|GetMaxSpeed)) false))

(event Input|AxisEvents|InputAxisMoveForward
  (params (AxisValue :type Float%20%28single-precision%29))
  ;[1 1 1] Movement
  (Pawn|Input|AddMovementInput (Transformation|GetActorForwardVector) (* AxisValue (Variables|Default|GetMaxSpeed)) false))

(fn ConstructionScript)