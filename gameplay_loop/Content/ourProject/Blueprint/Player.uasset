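; Player pawn with a sheep sprite mesh that moves on input and does a card-flip style spin.
; MoveForward and MoveRight add speed-scaled movement input, which Tick consumes as a swept local offset, and full axis deflection starts the spin.
; Spin advances yaw each tick independent of delta time, jumps from 90 to 270 degrees while swapping to the BackRight material, then resets after a full turn.
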(event EventBeginPlay)

(event Collision|EventActorBeginOverlap
  (params (OtherActor :type Actor%20Object%20Reference)))

(event EventTick
  (params (DeltaSeconds :type Float%20%28single-precision%29))
  ;[1 1 1] Tick
  (bind _returnvalue (Class|Pawn|ConsumeMovementInputVector))
  (Transformation|AddActorLocalOffset (* _returnvalue DeltaSeconds) true false)
  (if (Variables|Default|GetSpinning)
    (CallFunction|Spin (Variables|sprite|GetSheep) (Variables|Default|GetBack%20Right))))

(event Input|AxisEvents|InputAxisMoveRight
  (params (AxisValue :type Float%20%28single-precision%29))
  ;[1 1 1] Movement
  (Pawn|Input|AddMovementInput (Transformation|GetActorRightVector) (* AxisValue (Variables|Default|GetMaxSpeed)) false)
  (if (<= 1.0 AxisValue)
    (Variables|Default|SetSpinning true :!label _label)
    (elif (<= AxisValue -1.0)
      (goto _label))))

(event Input|AxisEvents|InputAxisMoveForward
  (params (AxisValue :type Float%20%28single-precision%29))
  ;[1 1 1] Movement
  (Pawn|Input|AddMovementInput (Transformation|GetActorForwardVector) (* AxisValue (Variables|Default|GetMaxSpeed)) false)
  (if (<= 1.0 AxisValue)
    (Variables|Default|SetSpinning true :!label _label)
    (elif (<= AxisValue -1.0)
      (goto _label))))

(fn ConstructionScript)

(fn Spin
  (params (Mesh :type Static%20Mesh%20Component%20Object%20Reference) (New%20Sprite :type Material%20Object%20Reference))
  (bind _output_get (Variables|Default|SetRotation (Math|Float|Max(Float) (Math|Float|Min(Float) (+ (Variables|Default|GetRotation) 1.0) 3.6e+02) 0.0)))
  (if (<= 9e+01 _output_get)
    (if (< _output_get 2.7e+02)
      (Variables|Default|SetRotation 2.7e+02)
      (Rendering|Material|SetMaterial Mesh 0 New%20Sprite)))
  (Transformation|SetRelativeRotation Mesh (Math|Rotator|MakeRotator 9e+01 0.0 (+ 9e+01 _output_get)) false false)
  ;[1 1 1] Check if spin is complete
  (if (<= 3.6e+02 _output_get)
    (Variables|Default|SetSpinning false)
    (Variables|Default|SetRotation 0.0)
    (else
      (Variables|Default|SetSpinning true))))